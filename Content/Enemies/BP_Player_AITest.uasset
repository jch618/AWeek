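; Test player character for exercising enemy AI, with debug keys and a timeline-driven over-the-shoulder zoom.
; Key 1 toggles a BP_BaseEnemy's AI controller between combat and passive; 2 launches a test grenade.
; T sphere-traces forward for pawns, applying damage and reporting it to AI damage sensing.
; TakeDamage forwards to DamageSystem, while the health getters and Heal are stubs returning zero.
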(event `Key|Two`
  (params (Key :type "Key Structure"))
  (:`Pressed`
    (bind _returnvalue (`|SpawnActorFromClass` "/Game/Enemies/BP_Grenade_AITest.BP_Grenade_AITest_C" (`KismetMathLibrary.MakeTransform` (`SceneComponent.K2_GetComponentLocation` (`self.GrenadeREF`)) (`self.K2_GetActorRotation`)) "Undefined" "MultiplyWithRoot" null null))
    (`PrimitiveComponent.SetPhysicsLinearVelocity` (`/Game/Enemies/BP_Grenade_AITest.Sphere` _returnvalue) (* (`KismetMathLibrary.GetDirectionUnitVector` (`self.K2_GetActorLocation`) (`self.K2_GetActorLocation` _returnvalue)) 600.0) false "None")))

(event `Key|One`
  (params (Key :type "Key Structure"))
  (:`Pressed`
    (bind _returnvalue (`GameplayStatics.GetActorOfClass` "/Game/Enemies/BP_BaseEnemy.BP_BaseEnemy_C"))
    (bind _asaic_base_enemy (cast `/Game/Enemies/AIC_BaseEnemy` (`AIBlueprintHelperLibrary.GetAIController` _returnvalue)))
    (`/Engine/EditorBlueprintResources/StandardMacros.FlipFlop`
      (:`A`
        (`/Game/Enemies/AIC_BaseEnemy.SetStateAsInCombat` _asaic_base_enemy self))
      (:`B`
        (`/Game/Enemies/AIC_BaseEnemy.SetStateAsPassive` _asaic_base_enemy)))))

(event `Key|T`
  (params (Key :type "Key Structure"))
  (bind _returnvalue (`self.K2_GetActorLocation`))
  (:`Pressed`
    (bind (_outhit _returnvalue_2) (`KismetSystemLibrary.SphereTraceSingleForObjects` :`Start` _returnvalue :`End` (+ _returnvalue (* (`self.GetActorForwardVector`) 100.0)) :`Radius` 20.0 :`ObjectTypes` (`|MakeArray` "ObjectTypeQuery3" :!type "EObjectTypeQuery Enum") :`DrawDebugType` "ForDuration" :`DrawTime` 0.5))
    (if _returnvalue_2
      (bind (_bblockinghit _binitialoverlap _time _distance _location _impactpoint _normal _impactnormal _physmat _hitactor) (`GameplayStatics.BreakHitResult` _outhit))
      (message `DamageAble.TakeDamage` _hitactor (make `DamageInfo` 10.0))
      (`AISense_Damage.ReportDamageEvent` _hitactor self 10.0 (`self.K2_GetActorLocation`)))))

(event `EnhancedInput|/Game/Player/Input/Actions/IA_Zoom`
  (params (ActionValue :type Boolean) (ElapsedSeconds :type "Float (double-precision)") (TriggeredSeconds :type "Float (double-precision)") (InputAction :type "InputAction Object Reference" :default "/Game/Player/Input/Actions/IA_Zoom.IA_Zoom"))
  (:`Started`
    (bind (_direction _maintrack) (`Timeline|ZoomTimline` :!label _label)
      (:`Update`
        (set `SpringArmComponent.TargetArmLength` (`KismetMathLibrary.Lerp` 400.0 250.0 _maintrack) (`self.CameraBoom`))
        (set `SpringArmComponent.SocketOffset` (`KismetMathLibrary.MakeVector` 0.0 (`KismetMathLibrary.Lerp` 0.0 100.0 _maintrack) (`KismetMathLibrary.Lerp` 0.0 30.0 _maintrack)) (`self.CameraBoom`)))))
  (:`Completed`
    (goto _label :!via `Reverse`)))

(fn `GetCurrentHealth`
  (returns (ReturnValue :type "Float (single-precision)"))
  (return 0.0))

(fn `GetMaxHealth`
  (returns (ReturnValue :type "Float (single-precision)"))
  (return 0.0))

(fn `Heal`
  (params (amount :type "Float (single-precision)"))
  (returns (ReturnValue :type "Float (single-precision)"))
  (return 0.0))

(fn `TakeDamage`
  (params (DamageInfo :type "DamageInfo Structure"))
  (returns (ReturnValue :type Boolean))
  (bind _returnvalue (`DamageAble.TakeDamage` (`self.DamageSystem`) DamageInfo))
  (return _returnvalue))

(fn `UserConstructionScript`)