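; Breakable structure in the enemies folder, apparently a test variant for AI, that takes damage through a DamageSystem.
; TakeDamage forwards the damage info to DamageSystem, prints a debug message and returns the result.
; The construction script binds an event to DamageSystem's OnDeath, and the BreakStructure event calls StructureBreak.
; GetCurrentHealth, GetMaxHealth and Heal are stubs that return zero.
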(event `BreakStructure`
  (`self.StructureBreak`))

(fn `GetCurrentHealth`
  (returns (ReturnValue :type "Float (single-precision)"))
  (return 0.0))

(fn `GetMaxHealth`
  (returns (ReturnValue :type "Float (single-precision)"))
  (return 0.0))

(fn `Heal`
  (params (amount :type "Float (single-precision)"))
  (returns (ReturnValue :type "Float (single-precision)"))
  (return 0.0))

(fn `TakeDamage`
  (params (DamageInfo :type "DamageInfo Structure"))
  (returns (ReturnValue :type Boolean))
  (bind _returnvalue (`DamageAble.TakeDamage` (`self.DamageSystem`) DamageInfo))
  (`KismetSystemLibrary.PrintString` "Structure Damaged")
  (return _returnvalue))

(fn `UserConstructionScript`
  (add `DamageSystemComponent.OnDeath` (`self.DamageSystem`) (`|CreateDelegate` :!event `StructureBreak`)))