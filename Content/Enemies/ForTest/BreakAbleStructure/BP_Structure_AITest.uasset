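; Test breakable structure in the enemy test content that takes damage through a DamageSystem component and destroys itself.
; At BeginPlay it sizes its Box component to half the Cube's local bounds size.
; TakeDamage forwards to DamageSystem, whose OnDeath is bound in the construction script.
; Structure_Destroyed deactivates the Box, then destroys the actor after a short delay; health, heal and attack-token functions are stubs.
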(event `self.ReceiveBeginPlay`
  (bind (_min _max) (`StaticMeshComponent.GetLocalBounds` (`self.Cube`)))
  (`BoxComponent.SetBoxExtent` (`self.Box`) (/ (- _max _min) 2.0) true))

(event `Structure_Destroyed`
  (`KismetSystemLibrary.PrintString` "Destroyed")
  (`ActorComponent.SetActive` (`self.Box`) false false)
  (`KismetSystemLibrary.Delay` 0.5)
  (`self.K2_DestroyActor`))

(fn `GetCurrentHealth`
  (returns (ReturnValue :type "Float (single-precision)"))
  (return 0.0))

(fn `GetIsDead`
  (returns (ReturnValue :type Boolean))
  (return false))

(fn `GetMaxHealth`
  (returns (ReturnValue :type "Float (single-precision)"))
  (return 0.0))

(fn `Heal`
  (params (amount :type "Float (single-precision)"))
  (returns (ReturnValue :type "Float (single-precision)"))
  (return 0.0))

(fn `ReserveAttackToken`
  (params (Amount :type Integer))
  (returns (ReturnValue :type Boolean))
  (return false))

(fn `TakeDamage`
  (params (DamageInfo :type "DamageInfo Structure"))
  (returns (ReturnValue :type Boolean))
  (bind _returnvalue (`DamageAble.TakeDamage` (`self.DamageSystem`) DamageInfo))
  (`KismetSystemLibrary.PrintString` "Damaged")
  (return _returnvalue))

(fn `UserConstructionScript`
  (add `DamageSystemComponent.OnDeath` (`self.DamageSystem`) (`|CreateDelegate` :!event `Structure_Destroyed`)))