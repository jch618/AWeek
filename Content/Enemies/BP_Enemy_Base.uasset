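; Base enemy character that routes incoming damage through a DamageSystem component and reacts to its death, block and response events.
; The default attack plays the "Attack" montage from the anim instance's map, sphere-traces forward on notify to hit non-enemy pawns, then signals attack end.
; Death stops the AI brain and switches the mesh to ragdoll.
; Block and damage responses only print, and health getters and Heal are stubs returning zero.
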(event `self.ReceiveBeginPlay`
  (bind _asaic_enemy_base (cast `/Game/Enemies/AIC_Enemy_Base` (`AIBlueprintHelperLibrary.GetAIController` self))
    (:`then`
      (set `self.AICEnemyBase` _asaic_enemy_base))
    (:`CastFailed`
      (`KismetSystemLibrary.PrintString` "There is No AIC Now" true true (struct :`R` 1.0 :`G` 0.020335 :`B` 0.160115 :`A` 1.0) 10.0))))

(event `DefaultAttack`
  (bind _returnvalue (`self.K2_GetActorLocation`))
  (bind _asaweek_character_anim_instance (cast `AWeekCharacterAnimInstance` (`SkeletalMeshComponent.GetAnimInstance` (`self.Mesh`))))
  (bind _notifyname (`|PlayMontage` (`self.Mesh`) (`BlueprintMapLibrary.Map_Find` (`AWeekCharacterAnimInstance.mMontageMap` _asaweek_character_anim_instance) "Attack"))
    (:`OnCompleted`
      (`self.OnAttackEnd` :!label _label))
    (:`OnInterrupted`
      (goto _label))
    (:`OnNotifyBegin`
      (switch `name` _notifyname
        (:`Smash`
          (bind (_outhit _returnvalue_2) (`KismetSystemLibrary.SphereTraceSingleForObjects` :`Start` _returnvalue :`End` (+ _returnvalue (* (`self.GetActorForwardVector`) 200.0)) :`Radius` 20.0 :`ObjectTypes` (`|MakeArray` "ObjectTypeQuery3" :!type "EObjectTypeQuery Enum") :`DrawDebugType` "ForDuration"))
          (if _returnvalue_2
            (bind (_bblockinghit _binitialoverlap _time _distance _location _impactpoint _normal _impactnormal _physmat _hitactor) (`GameplayStatics.BreakHitResult` _outhit))
            (cast `/Game/Enemies/BP_Enemy_Base` _hitactor
              (:`CastFailed`
                (message `DamageAble.TakeDamage` _hitactor (struct))
                (`KismetSystemLibrary.PrintString` (`KismetSystemLibrary.GetDisplayName` _hitactor))))))))))

(event `Death`
  (bind _mesh (`self.Mesh`))
  (`BrainComponent.StopLogic` (`AIController.BrainComponent` (`self.AICEnemyBase`)) "")
  (`PrimitiveComponent.SetSimulatePhysics` _mesh true)
  (`PrimitiveComponent.SetCollisionEnabled` _mesh "QueryAndPhysics")
  (`KismetSystemLibrary.PrintString` "Death")
  (`PrimitiveComponent.SetCollisionProfileName` (`self.Mesh`) "Ragdoll" true)
  (`PrimitiveComponent.SetCollisionResponseToChannel` _mesh "ECC_Pawn" "ECR_Ignore")
  (`PrimitiveComponent.SetCollisionResponseToChannel` _mesh "ECC_Camera" "ECR_Ignore")
  (`PrimitiveComponent.SetCollisionEnabled` (`self.CapsuleComponent`) "NoCollision"))

(event `Block`
  (params (CanBeParried :type Boolean))
  (`KismetSystemLibrary.PrintString` "Block"))

(event `DamageResponse`
  (params (DamageResponse :type "EDamageResponse Enum" :default "None"))
  (`KismetSystemLibrary.PrintString` (`|GetEnumeratorNameAsString` DamageResponse)))

(fn `GetCurrentHealth`
  (returns (ReturnValue :type "Float (single-precision)"))
  (return 0.0))

(fn `GetMaxHealth`
  (returns (ReturnValue :type "Float (single-precision)"))
  (return 0.0))

(fn `Heal`
  (params (amount :type "Float (single-precision)"))
  (returns (ReturnValue :type "Float (single-precision)"))
  (return 0.0))

(fn `TakeDamage`
  (params (DamageInfo :type "DamageInfo Structure"))
  (returns (ReturnValue :type Boolean))
  (bind _returnvalue (`DamageAble.TakeDamage` (`self.DamageSystem`) DamageInfo))
  (return _returnvalue))

(fn `UserConstructionScript`
  (bind _damagesystem (`self.DamageSystem`))
  (add `DamageSystemComponent.OnDeath` _damagesystem (`|CreateDelegate` :!event `Death`))
  (add `DamageSystemComponent.OnBlocked` _damagesystem (`|CreateDelegate` :!event `Block`))
  (add `DamageSystemComponent.OnDamageResponse` _damagesystem (`|CreateDelegate` :!event `DamageResponse`)))