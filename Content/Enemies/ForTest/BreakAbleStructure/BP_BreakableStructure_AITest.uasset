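; Test breakable structure for enemy AI that takes damage through a DamageSystem component and exposes a BreakStructure event that calls StructureBreak.
; The construction script binds a handler to the component's OnDeath.
; TakeDamage forwards to the component and spawns a short-lived bullet-hole decal, with no hit location or normal wired in.
; Health queries, Heal and ReserveAttackToken are stubs returning zero or false.
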(event `BreakStructure`
  (`self.StructureBreak`))

(fn `GetCurrentHealth`
  (returns (ReturnValue :type "Float (single-precision)"))
  (return 0.0))

(fn `GetIsDead`
  (returns (ReturnValue :type Boolean))
  (return false))

(fn `GetMaxHealth`
  (returns (ReturnValue :type "Float (single-precision)"))
  (return 0.0))

(fn `Heal`
  (params (amount :type "Float (single-precision)"))
  (returns (ReturnValue :type "Float (single-precision)"))
  (return 0.0))

(fn `ReserveAttackToken`
  (params (Amount :type Integer))
  (returns (ReturnValue :type Boolean))
  (return false))

(fn `TakeDamage`
  (params (DamageInfo :type "DamageInfo Structure"))
  (returns (ReturnValue :type Boolean))
  (locals (DInfo :type "DamageInfo Structure"))
  (bind _output_get (set `local.DInfo` DamageInfo))
  (bind _returnvalue (`DamageAble.TakeDamage` (`self.DamageSystem`) _output_get))
  (bind _returnvalue_2 (`GameplayStatics.SpawnDecalAtLocation` "/Game/Enemies/ForTest/M_bullethole.M_bullethole" (5.0 5.0 3.0) (0.0 0.0 0.0) (`KismetMathLibrary.Conv_VectorToRotator` (0.0 0.0 0.0)) 5.0))
  (`DecalComponent.SetFadeScreenSize` _returnvalue_2 0.001)
  (return _returnvalue))

(fn `UserConstructionScript`
  (add `DamageSystemComponent.OnDeath` (`self.DamageSystem`) (`|CreateDelegate` :!event `StructureBreak`)))