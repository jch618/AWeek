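; BP_PatrolRoute is an enemy patrol route that exposes the points of a spline as world-space patrol destinations.
; BeginPlay caches the last spline point index, and GetSplinePointAsWorldPosition returns the location of the current patrol index.
; IncrementPatrolRoute steps that index and flips its direction at either end, so the route runs back and forth instead of looping.
; The index and direction live on the route itself.
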(event `self.ReceiveBeginPlay`
  (set `self.MaxIdxofSplinePoint` (- (`SplineComponent.GetNumberOfSplinePoints` (`self.Spline`)) 1)))

(event `IncrementPatrolRoute`
  (bind _output_get (set `self.PatrolIdx` (+ (`self.PatrolIdx`) (`self.PatrolDirection`))))
  (if (or (== _output_get (`self.MaxIdxofSplinePoint`)) (== _output_get 0))
    (set `self.PatrolDirection` (* (`self.PatrolDirection`) -1))))

(fn `GetSplinePointAsWorldPosition`
  (returns (Location :type "Vector Structure"))
  (return (`SplineComponent.GetLocationAtSplinePoint` (`self.Spline`) (`self.PatrolIdx`) "World")))

(fn `UserConstructionScript`)